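; Racing game mode that runs a checkpoint time-trial with a countdown and a time limit.
; On BeginPlay it binds every BP_Checkpoint, then starts the countdown that arms the out-of-time timer.
; Regular checkpoints extend time by re-arming the timer with remaining plus bonus seconds; the finish line clears it.
; Both winning and timeout call GameFinish with false, which only disables player input.
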(event `Start Countdown`
  (`KismetSystemLibrary.Delay` (`self.StartCountdownDuration`))
  (`self.Game Start`))

(event `Game Start`
  (bind _returnvalue (`KismetSystemLibrary.K2_SetTimerDelegate` (delegate `Loose?OutofTime`) (`self.StartTimerDuration`)))
  (set `self.TimeRemainTimer` _returnvalue))

(event `Loose?OutofTime`
  (`self.Game Finish` false))

(event `Win`
  (`KismetSystemLibrary.K2_ClearAndInvalidateTimerHandle` (`self.TimeRemainTimer`))
  (`self.Game Finish` false))

(event `self.ReceiveBeginPlay`
  (`|ExecutionSequence`
    (:`then_0`
      (bind _outactors (`GameplayStatics.GetAllActorsOfClass` "/Game/Bryan/BP_Checkpoint.BP_Checkpoint_C"))
      (for _array_element _outactors
        (if (`/Game/Bryan/BP_Checkpoint.IsFinishLine` _array_element)
          (add `/Game/Bryan/BP_Checkpoint.OnCheckpointCrossed` _array_element (delegate `Win`))
          (else
            (add `/Game/Bryan/BP_Checkpoint.OnCheckpointCrossedTime` _array_element (`|CreateDelegate` :!event `CheckpointCross`))))))
    (:`then_1`
      (`self.Start Countdown`))))

(event `Game Finish`
  (params (Win :type Boolean))
  (`self.DisableInput` (`GameplayStatics.GetPlayerPawn` 0) (`GameplayStatics.GetPlayerController` 0)))

(event `CheckpointCross`
  (params (TimeToAdd :type Integer))
  (`self.Add Time to Timer` TimeToAdd))

(event `PreRace`)

(fn `Add Time to Timer`
  (params (TimeToAdd :type Integer))
  (bind _returnvalue (`KismetSystemLibrary.K2_SetTimerDelegate` (`|CreateDelegate` :!event `Loose?OutofTime`) (+ TimeToAdd (`KismetSystemLibrary.K2_GetTimerRemainingTimeHandle` (`self.TimeRemainTimer`)))))
  (set `self.TimeRemainTimer` _returnvalue))

(fn `UserConstructionScript`)